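; FPS player controller Blueprint that manages the client's HUD widgets through Blueprint wrapper events.
; It creates the in-game and score UIs once, registers the former with BP_GameState, and refreshes team and rival score bars.
; Tab held shows the scoreboard widget, if one exists.
; Scoreboard build and per-player stat update events are empty; their two-team, row-per-player logic, highlighting the local player, remains disconnected.
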(event `self.UpdateScoreUIBlueprint`
  ;[1 1 1] ScoreUI
  (`self.UpdateScore`))

(event `UpdateScore`
  (bind _scoreui (`self.ScoreUI`))
  ;[1 1 1] ScoreUI
  (`/Engine/EditorBlueprintResources/StandardMacros.IsValid` (`self.ScoreUI`)
    (:`Is Valid`
      (`ProgressBar.SetPercent` (`/Game/UI/ScoreUI.MyScore` _scoreui) (`self.TeamScorePercent`))
      (`ProgressBar.SetPercent` (`/Game/UI/ScoreUI.EnemyScore` _scoreui) (`self.RivalScorePercent`)))))

(event `self.TriggerAddAliveUIBlueprint`
  ;[1 1 1] GameUI
  (`self.AddGameUIToClient`))

(event `Key|Tab`
  (params (Key :type "Key Structure" :default "AnyKey"))
  (:`Pressed`
    (`self.ShowScoreBoard`))
  (:`Released`
    (`self.RemoveScoreBoard`)))

(event `AddGameUIToClient`
  ;[1 1 1] GameUI
  (`/Engine/EditorBlueprintResources/StandardMacros.IsValid` (`self.InGameUI`)
    (:`Is Not Valid`
      (bind _returnvalue (`|CreateWidget` "/Game/UI/InGameUI.InGameUI_C"))
      (bind _output_get (set `self.InGameUI` _returnvalue))
      (bind _asbp_game_state (cast `/Game/Blueprints/BP_GameState` (`GameplayStatics.GetGameState`)))
      (set `/Game/Blueprints/BP_GameState.UI` _returnvalue _asbp_game_state)
      (`UserWidget.AddToViewport` _output_get 0)
      (bind _returnvalue_2 (`|CreateWidget` "/Game/UI/ScoreUI.ScoreUI_C"))
      (bind _output_get_2 (set `self.ScoreUI` _returnvalue_2))
      (`UserWidget.AddToViewport` _output_get_2 1))))

(event `ShowScoreBoard`
  (bind _scoreboardui (`self.ScoreBoardUI`))
  (`/Engine/EditorBlueprintResources/StandardMacros.IsValid` _scoreboardui
    (:`Is Valid`
      (`Widget.SetVisibility` _scoreboardui "Visible"))))

(event `RemoveScoreBoard`
  (bind _scoreboardui (`self.ScoreBoardUI`))
  (`/Engine/EditorBlueprintResources/StandardMacros.IsValid` _scoreboardui
    (:`Is Valid`
      (`Widget.SetVisibility` _scoreboardui "Hidden"))))

(event `self.AddScoreBoardUIBlueprint`
  ;[1 1 1] base scoreboard
  (`self.AddScoreBoardToClient`))

(event `AddScoreBoardToClient`
  ;[1 1 1] base scoreboard
)

(event `UpdatePlayerStats`
  ;[1 1 1] UpdateScoreBoard
)

(event `self.UpdateScoreBoardUIBlueprint`
  ;[1 1 1] UpdateScoreBoard
  (`self.UpdatePlayerStats`))

(fn `UserConstructionScript`)